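; GM_Vats is a manager Blueprint, apparently the game mode, that scatters randomized buildings for multiplayer and handles music.
; Five seconds after BeginPlay, letting players connect, it builds a jittered grid around each "SpawnBuilding" actor through the first player's BP_Player ServerObstacle call, randomizing scale and material.
; The Y index (Hauteur) never resets, so later grids drift outward.
; A music event stops any valid sound, otherwise plays the chosen track.
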(event EventBeginPlay
  ;[0.15 0.15 0.15 0.5] Initialisation du premier joueur
  (bind _asbp_player (Utilities|Casting|CastToBP_Player (Game|GetPlayerCharacter 0)))
  (Variables|Default|SetRef%20BP%20Player _asbp_player)
  ;[0.15 0.15 0.15 0.5 13] On laisser du temps pour que tous les joueur puisse ce connecter
  (Utilities|FlowControl|Delay 5.0)
  ;[0.15 0.15 0.15 0.5] Placement de tous les building en multijoueur
  (bind _outactors (Actor|GetAllActorsOfClasswithTag "/Script/Engine.Actor" "SpawnBuilding"))
  (for _array_element _outactors
    (CallFunction|FunctionSpawnActor _array_element)))

(event EventFunctionSelectionMusique
  (params (ChoisMusique :type Sound%20Base%20Object%20Reference))
  ;[0.15 0.15 0.15 0.5] Choix de musique non enregistrer
  (bind _sound (Variables|Default|GetSound)
    (:then
      (Audio|Components|Audio|Stop _sound))
    (:else
      (bind _returnvalue (Audio|SpawnSound2D ChoisMusique 1.0 1.0 0.0 0))
      (Variables|Default|SetSound _returnvalue))))

(fn ConstructionScript)

(fn FunctionSpawnActor
  (params (Cible :type Actor%20Object%20Reference))
  (Utilities|IsValid Cible
    (:Is%20Valid
      (for _index (range 0 5)
        (for _index_2 (range 0 5)
          (Default|Server:Obstacle (Variables|Default|GetRef%20BP%20Player) (Math|Transform|MakeTransform (+ (Transformation|GetActorLocation Cible) (Math|Vector|MakeVector (* (LocalVariables|GetLongueur) (Math|Random|RandomFloatinRange 5e+02 1.5e+03)) (* (LocalVariables|GetHauteur) (Math|Random|RandomFloatinRange 5e+02 1.5e+03)) 0.0))) (Math|Vector|MakeVector (Math|Random|RandomFloatinRange 0.3 1.5) (Math|Random|RandomFloatinRange 0.3 1.5) (Math|Random|RandomFloatinRange 5.0 15.0)) (Math|Random|RandomIntegerinRange 0 2))
          (Math|Integer|IncrementInt (LocalVariables|GetLongueur)))
        (Math|Integer|IncrementInt (LocalVariables|GetHauteur)
          (:%20%20
            (LocalVariables|SetLongueur 0)))))))