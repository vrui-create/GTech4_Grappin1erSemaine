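; BP_Piece is a collectible coin that adds to the score of the player who picks it up.
; A Timeline started on BeginPlay animates the mesh's relative height and yaw.
; The first BP_Player overlap, gated by DoOnce, calls the coin-add event on that player's PS_PlayerState, then destroys the piece after a short delay.
; If its linked obstacle reference is valid, the pickup also tells that obstacle to spawn a piece.
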(event OnComponentBeginOverlap(StaticMesh)
  (params (OverlappedComponent :type Primitive%20Component%20Object%20Reference) (OtherActor :type Actor%20Object%20Reference) (OtherComp :type Primitive%20Component%20Object%20Reference) (OtherBodyIndex :type Integer) (bFromSweep :type Boolean) (SweepResult :type Hit%20Result%20Structure%20%28by%20ref%29))
  (bind (_asbp_player _bsuccess) (Utilities|Casting|CastToBP_Player OtherActor))
  (if _bsuccess
    (Utilities|FlowControl|DoOnce false
      (:Completed
        (CallFunction|FunctionAddScoretoStatePlayer _asbp_player)
        (Utilities|FlowControl|Delay 0.1)
        (Actor|DestroyActor)))))

(event EventBeginPlay
  (bind (_direction _relativelocate_z _relativerotation_z) (Timeline|Timeline PlayFromStart)
    (:Update
      (Transformation|SetRelativeLocationAndRotation (Variables|Default|GetStaticMesh) (Math|Vector|MakeVector 0.0 0.0 _relativelocate_z) (Math|Rotator|MakeRotator 0.0 0.0 _relativerotation_z) true false))))

(fn ConstructionScript)

(fn FunctionAddScoretoStatePlayer
  (params (Player :type BP%20Player%20Object%20Reference))
  (bind _asps_player_state (Utilities|Casting|CastToPS_PlayerState (Variables|/Script/Engine.Pawn|GetPlayerState Player))
    (:then
      (Default|CEAddCoint:Server _asps_player_state)
      (bind _ref_obstacle (Variables|Default|GetREF_Obstacle)
        (:then
          (Default|CESpawnPiece _ref_obstacle))
        (:else)))
    (:CastFailed
      (Development|PrintString "Hello"))))