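; BP_Placement_Obstcale is a placer actor that scatters BP_Obstacle actors over a randomized horizontal grid when play begins.
; FunctionPlacementDesObstacle runs nested loops over column (Longueur) and row (Hauteur) counters, passing each offset to FunctionSpawnObstacle, which adds the actor's location.
; Each axis offset is the index times a fresh random spacing, so scatter widens with distance and zero indices stay aligned with the actor.
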(event EventBeginPlay
  (CallFunction|FunctionPlacementDesObstacle))

(fn ConstructionScript)

(fn FunctionSpawnObstacle
  (params (Bruh :type Vector))
  (Game|SpawnActorfromClass "/Game/Vats/PROG/Obstacle/BP_Obstacle.BP_Obstacle_C" (Math|Transform|MakeTransform (+ Bruh (Transformation|GetActorLocation)) "0, 0, 0" "1.000000,1.000000,1.000000") "Undefined" "MultiplyWithRoot" 0 0))

(fn FunctionPlacementDesObstacle
  (for _index (range 0 5)
    (for _index_2 (range 0 5)
      (CallFunction|FunctionSpawnObstacle (Math|Vector|MakeVector (* (Variables|Default|GetLongueur) (Math|Random|RandomFloatinRange 5e+02 1.5e+03)) (* (Variables|Default|GetHauteur) (Math|Random|RandomFloatinRange 5e+02 1.5e+03)) 0.0))
      (Math|Integer|IncrementInt (Variables|Default|GetLongueur)))
    (Math|Integer|IncrementInt (Variables|Default|GetHauteur)
      (:%20%20
        (Variables|Default|SetLongueur 0)))))