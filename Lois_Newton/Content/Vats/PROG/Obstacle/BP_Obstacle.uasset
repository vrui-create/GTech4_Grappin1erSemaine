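; BP_Obstacle is an obstacle actor that randomizes its shape at BeginPlay and spawns a BP_Piece pickup around itself.
; It gives the Obstacle a tall random scale and the Plateforme a thin, wider one, then resets Sphere's world scale.
; The piece receives a reference to the obstacle, attaches to Sphere and takes a random corner offset and height.
; A DoOnce, reset after a short delay, throttles repeated spawn calls.
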(event Custom|CE_SpawnPiece
  (Utilities|FlowControl|DoOnce false
    (:Completed
      (bind _returnvalue (Game|SpawnActorfromClass "/Game/Vats/PROG/Collectif/BP_Piece.BP_Piece_C" (Math|Transform|MakeTransform (Transformation|GetActorLocation) "0, 0, 0" "1.000000,1.000000,1.000000") "Undefined" "MultiplyWithRoot" 0 self 0))
      (bind _output_get (Variables|Default|SetPiece _returnvalue))
      (Transformation|AttachComponentToComponent _output_get (Variables|Default|GetSphere) "None" "KeepRelative" "KeepRelative" "KeepRelative" true)
      (Transformation|SetActorRelativeLocation (Variables|Default|GetPiece) (Math|Vector|MakeVector (select (Math|Random|RandomBool) 3e+02 -3e+02) (select (Math|Random|RandomBool) 3e+02 -3e+02) (Math|Random|RandomFloatinRange -1.5e+03 2e+02)) false true)
      (Utilities|FlowControl|Delay 0.5)
      (CallFunction|CEResetDoOnce))))

(event Custom|CE_Reset%20Do%20Once
  (Utilities|FlowControl|DoOnce false) ; enters at Reset
)

(event EventBeginPlay
  (CallFunction|FunctionGestionTaille)
  (CallFunction|CESpawnPiece))

(fn ConstructionScript)

(fn FunctionGestionTaille
  (bind _returnvalue (Math|Random|RandomFloatinRange 0.3 1.5))
  (bind _returnvalue_2 (Math|Random|RandomFloatinRange 0.3 1.5))
  (Transformation|SetRelativeScale3D (Variables|Default|GetObstacle) (Math|Vector|MakeVector _returnvalue _returnvalue_2 (Math|Random|RandomFloatinRange 5.0 15.0)))
  (Transformation|SetRelativeScale3D (Variables|Default|GetPlateforme) (Math|Vector|MakeVector (+ _returnvalue 1.0) (+ _returnvalue_2 1.0) 0.1))
  (Transformation|SetWorldScale3D (Variables|Default|GetSphere) "1.000000,1.000000,1.000000"))