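; Player controller for the multiplayer lobby, which shows the lobby HUD with the mouse cursor and handles session hosting, search and joining.
; Custom events open the tutorial map or create a four-connection session that loads the game level on success.
; Session search clears the HUD list, fills it with one widget per lobby result and tracks progress in a SearchPlayer flag.
; A separate event joins a given search result.
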(event Custom|CE_FindSession
  (Widget|Panel|ClearChildren (Variables|/Game/Vats/PROG/Multijoueur/HUD_Lobby.HUD_Lobby_C|GetVerticalBox_Session (Variables|Default|GetHUD)))
  (Variables|Default|SetSearchPlayer true)
  (bind _results (|FindSessions self 0 false true)
    (:OnSuccess
      (for _array_element _results
        (bind _returnvalue (UserInterface|CreateWidget "/Game/Vats/PROG/Multijoueur/HUD_Session.HUD_Session_C" 0 _array_element))
        (UserInterface|Viewport|AddtoViewport _returnvalue 0)
        (Widget|Panel|AddChild (Variables|/Game/Vats/PROG/Multijoueur/HUD_Lobby.HUD_Lobby_C|GetVerticalBox_Session (Variables|Default|GetHUD)) _returnvalue))
      (Variables|Default|SetSearchPlayer false))))

(event Custom|CE_CreationSession
  (|Session self 4 false true
    (:OnSuccess
      (Game|OpenLevel(byObjectReference) "/Game/Vats/MAP/LEVEL_GAME.LEVEL_GAME"))))

(event Custom|CE_OPEN_MAP_TUTO
  (Game|OpenLevel(byObjectReference) "/Game/Vats/MAP/MAP_TUTO.MAP_TUTO"))

(event Custom|CE_JoindreSession
  (params (SearchResult :type Blueprint%20Session%20Result%20Structure%20%28by%20ref%29))
  (|JoinSession self SearchResult))

(event EventBeginPlay
  (bind _returnvalue (UserInterface|CreateWidget "/Game/Vats/PROG/Multijoueur/HUD_Lobby.HUD_Lobby_C" self))
  (bind _output_get (Variables|Default|SetHUD _returnvalue))
  (UserInterface|Viewport|AddtoViewport _output_get 0)
  (Variables|Default|SetbShowMouseCursor true))

(fn ConstructionScript)