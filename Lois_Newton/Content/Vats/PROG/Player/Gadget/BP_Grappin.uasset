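; BP_Grappin is the player's grappling hook gadget, pulling the player toward it once it hits something.
; On BeginPlay it attaches its cable end to the player's Sphering component and closes a Tick gate.
; A Sphere hit on anything but the player opens the gate, applying impulses every frame toward the hook and along the camera's forward vector.
; Disconnected velocity debug and FOV code remains unused.
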(event OnComponentHit(Sphere)
  (params (HitComponent :type Primitive%20Component%20Object%20Reference) (OtherActor :type Actor%20Object%20Reference) (OtherComp :type Primitive%20Component%20Object%20Reference) (NormalImpulse :type Vector :default "0, 0, 0") (Hit :type Hit%20Result%20Structure%20%28by%20ref%29))
  (if (!= OtherActor (Variables|Default|GetRefPlayer))
    (Utilities|FlowControl|Gate true) ; enters at Open
  ))

(event EventBeginPlay
  (CallFunction|FunctionAttacherPlayer)
  (Utilities|FlowControl|Gate true) ; enters at Close
)

(event EventTick
  (params (DeltaSeconds :type Float%20%28single-precision%29))
  (Utilities|FlowControl|Gate true
    (:Exit
      (Variables|Default|GetRefPlayer
        (:then
          (Transformation|SetWorldRotation (Variables|Default|GetSphere) (Math|Rotator|FindLookatRotation (Transformation|GetActorLocation self) (Transformation|GetActorLocation (Variables|Default|GetRefPlayer))) false false)
          (Physics|AddImpulse (Variables|/Script/Engine.Character|GetCharacterMovement (Variables|Default|GetRefPlayer)) (* (Math|Vector|GetForwardVector (Variables|Default|GetSphere)) (Math|Conversions|ToVector(Float) -2e+03)) false)
          (Physics|AddImpulse (Variables|/Script/Engine.Character|GetCharacterMovement (Variables|Default|GetRefPlayer)) (* (Math|Vector|GetForwardVector (Variables|/Game/Vats/PROG/Player/BP_Player.BP_Player_C|GetCamera (Variables|Default|GetRefPlayer))) (Math|Conversions|ToVector(Float) 1e+03)) false))
        (:else
          (Development|PrintString "Hello"))))))

(fn ConstructionScript)

(fn FunctionAttacherPlayer
  (bind _refplayer (Variables|Default|GetRefPlayer)
    (:then
      (Class|CableComponent|SetAttachEndtoComponent (Variables|Default|GetCable) (Variables|/Game/Vats/PROG/Player/BP_Player.BP_Player_C|GetSphering _refplayer) "None"))
    (:else)))