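; Multiplayer player character with grappling hook, cooldown dash, double jump, speed-boost impulses and object interaction.
; Impulses and obstacle spawns pass through Server-to-Client RPC pairs so client players can use them.
; Capsule hits and sphere overlaps turn dashes or high-speed impacts into PlayerState health loss, with timelines driving feedback, invincibility and death-to-respawn.
; BeginPlay waits five seconds before adding input mapping and the HUD.
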(event OnComponentBeginOverlap(Sphering)
  (params (OverlappedComponent :type Primitive%20Component%20Object%20Reference) (OtherActor :type Actor%20Object%20Reference) (OtherComp :type Primitive%20Component%20Object%20Reference) (OtherBodyIndex :type Integer) (bFromSweep :type Boolean) (SweepResult :type Hit%20Result%20Structure%20%28by%20ref%29))
  ;[0 0 0 0.5 50] ALL Gestion des Degats
  ;;[0 0 0 0.5] Gestion dash, et infliger au ennemie ou au joueur
  (CallFunction|FunctionVerifieLaVelocity OtherActor))

(event OnComponentHit(CapsuleComponent)
  (params (HitComponent :type Primitive%20Component%20Object%20Reference) (OtherActor :type Actor%20Object%20Reference) (OtherComp :type Primitive%20Component%20Object%20Reference) (NormalImpulse :type Vector :default "0, 0, 0") (Hit :type Hit%20Result%20Structure%20%28by%20ref%29))
  ;[0 0 0 0.5 50] Gestion des mécaniquedes input
  ;;[0.15 0.15 0.15 0.5] Input Basic Des déplacement de personnage mes aussi
  (Class|BPIPlayer|FunctionDoubleJump(Message) self false)
  (CallFunction|FunctionVerifieLaVelocity OtherActor))

(event Custom|Client%20:%20SpawnPiece
  (params (SpawnTransform :type Transform) (REF_Obstacle :type BP%20Obstacle%20Object%20Reference) (InputPin :type BP%20Piece%20Object%20Reference))
  ;[0 0 0 0.5 50] Gestion placement D'objet dans le monde. Elle es gérer dans le GameMode XD
  ;;[0.15 0.002911 0 0.5] Ce code permet de synchroniser l'invocation des piece en multijoueur, pour le moment elle est désactiver en raison de probléme téchnique
  (Game|SpawnActorfromClass "/Game/Vats/PROG/Objet/BP_Piece.BP_Piece_C" SpawnTransform "Undefined" "MultiplyWithRoot" 0 REF_Obstacle 0)
  (Utilities|IsValid InputPin
    (:Is%20Valid
      (Actor|DestroyActor InputPin))))

(event Custom|Server%20:%20SpawnPiece
  (params (SpawnTransform :type Transform) (REF_Obstacle :type BP%20Obstacle%20Object%20Reference) (REF_Piece :type BP%20Piece%20Object%20Reference))
  (bind (_location _rotation _scale) (Math|Transform|BreakTransform SpawnTransform))
  ;[0 0 0 0.5 50] Gestion placement D'objet dans le monde. Elle es gérer dans le GameMode XD
  ;;[0.15 0.002911 0 0.5] Ce code permet de synchroniser l'invocation des piece en multijoueur, pour le moment elle est désactiver en raison de probléme téchnique
  (CallFunction|Client:SpawnPiece (Math|Transform|MakeTransform (+ _location (Math|Vector|MakeVector (select (Math|Random|RandomBool) 3e+02 -3e+02) (select (Math|Random|RandomBool) 3e+02 -3e+02) (Math|Random|RandomFloatinRange -1.5e+03 2e+02))) _rotation _scale) REF_Obstacle REF_Piece))

(event Custom|ResetDoONce%20Damage
  ;[0 0 0 0.5 50] ALL Gestion des Degats
  ;;[0 0 0 0.5] Gestion des dégats de sois même
  (Utilities|FlowControl|DoOnce false) ; enters at Reset
)

(event Custom|CE_Respawn
  (bind _ps_player_state (Variables|UseHUD|GetPS%20Player%20State))
  ;[0 0 0 0.5 50] ALL Gestion des Degats
  ;;[0 0 0 0.5] Gestion des dégats de sois même
  ;;;[0.15 0.15 0.15 0.5] Remêttre le joueur en place
  (bind _asbp_player_controller (Utilities|Casting|CastToBP_PlayerController (Pawn|GetController)))
  (Input|EnableInput self _asbp_player_controller)
  (bind _outactors (Actor|GetAllActorsOfClasswithTag "/Script/Engine.Actor" "Respawn"))
  (for _array_element _outactors
    _)
  (Transformation|SetActorLocationAndRotation self (.location (Transformation|GetActorTransform _array_element)) (.rotation (Transformation|GetActorTransform _array_element)))
  (Camera|SetFieldOfView (Variables|Default|GetCamera) 9e+01)
  (bind _ref_hud (Variables|UseHUD|GetREF_HUD)
    (:then
      (Variables|/Script/UMG.Border|SetBrushColor (Variables|/Game/Vats/PROG/Player/InfosPlayer/HUD_Player.HUD_Player_C|GetBorder_FeedBack_Degat _ref_hud) (Utilities|Struct|MakeLinearColor 0.0 0.0 0.0 0.0))
      (Variables|/Game/Vats/PROG/Player/InfosPlayer/PS_PlayerState.PS_PlayerState_C|SetPv_Joueur _ps_player_state (Variables|/Game/Vats/PROG/Player/InfosPlayer/PS_PlayerState.PS_PlayerState_C|GetPvMax_Joueur _ps_player_state)))
    (:else)))

(event Custom|Server%20:%20GrappinImpulsionPlayer
  (params (ForwardActor :type Vector))
  ;[0 0 0 0.5 50] Gestion des mécaniquedes input
  ;;[0.15 0.15 0.15 0.5] Mécanique Grappin
  ;;;[0.15 0.15 0.15 0.5] Ce code permet d'attirer le joueur vers le grappin et impulser on direction de la camera, ATTENTION ceci ce répéter avec l'évent Tick du BP_Grappin
  (CallFunction|Client:GrappinImpulsionPlayer ForwardActor))

(event Custom|Client%20:%20GrappinImpulsionPlayer
  (params (ForwardActor :type Vector))
  ;[0 0 0 0.5 50] Gestion des mécaniquedes input
  ;;[0.15 0.15 0.15 0.5] Mécanique Grappin
  ;;;[0.15 0.15 0.15 0.5] Ce code permet d'attirer le joueur vers le grappin et impulser on direction de la camera, ATTENTION ceci ce répéter avec l'évent Tick du BP_Grappin
  (Physics|AddImpulse (Variables|Character|GetCharacterMovement) ForwardActor false)
  (Physics|AddImpulse (Variables|Character|GetCharacterMovement) (* (Math|Vector|GetForwardVector (Variables|Default|GetCamera)) (Math|Conversions|ToVector(Float) 1e+03)) false))

(event Custom|FIN_JEUX
  ;[0 0 0 0.5] Ce code permet de désactiver le joueur de tout mouvement
  (bind _asbp_player_controller (Utilities|Casting|CastToBP_PlayerController (Pawn|GetController)))
  (Input|DisableInput _asbp_player_controller))

(event Custom|Client%20:%20Dashing
  (params (Impulse :type Vector))
  ;[0 0 0 0.5 50] Gestion des mécaniquedes input
  ;;[0.15 0.15 0.15 0.5] Mécanique Dashing Terminer
  ;;;[0.15 0.15 0.15 0.5 15] Permet au 2éme joueur d'utiliser l'impulsion, Unreal autoriser l'impulsion du Joueur 2 qu'a condition que le serveur soit encourant de la manoeuvre
  (Physics|AddImpulse (Variables|Character|GetCharacterMovement) Impulse true))

(event Custom|Server%20:%20Dashing
  (params (Impulse :type Vector))
  ;[0 0 0 0.5 50] Gestion des mécaniquedes input
  ;;[0.15 0.15 0.15 0.5] Mécanique Dashing Terminer
  ;;;[0.15 0.15 0.15 0.5 15] Permet au 2éme joueur d'utiliser l'impulsion, Unreal autoriser l'impulsion du Joueur 2 qu'a condition que le serveur soit encourant de la manoeuvre
  (CallFunction|Client:Dashing Impulse))

(event Custom|Server%20:%20Obstacle
  (params (SpawnTransform :type Transform) (Server%20:%20ScaleObject :type Vector) (Server%20:%20IntegrationMaterial :type Integer))
  ;[0 0 0 0.5 50] Gestion placement D'objet dans le monde. Elle es gérer dans le GameMode XD
  ;;[0.1486 0.15 0 0.5] Ce code permet de synchronisation l'invoque des obstacle ou building dans le monde dans le multijoueur
  (CallFunction|Client:Obstacle SpawnTransform Server%20:%20ScaleObject Server%20:%20IntegrationMaterial))

(event Custom|Client%20:%20Obstacle
  (params (SpawnTransform :type Transform) (Server%20:%20ScaleObject :type Vector) (Server%20:%20IntegrationMaterial :type Integer))
  ;[0 0 0 0.5 50] Gestion placement D'objet dans le monde. Elle es gérer dans le GameMode XD
  ;;[0.1486 0.15 0 0.5] Ce code permet de synchronisation l'invoque des obstacle ou building dans le monde dans le multijoueur
  (Game|SpawnActorfromClass "/Game/Vats/PROG/Objet/BP_Obstacle.BP_Obstacle_C" SpawnTransform "Undefined" "MultiplyWithRoot" 0 Server%20:%20ScaleObject Server%20:%20IntegrationMaterial 0))

(event Custom|Client%20:%20Impulse%20Speed%20Runner
  (params (DirectionImpulse :type Vector))
  ;[0 0 0 0.5 50] Gestion des mécaniquedes input
  ;;[0.15 0.15 0.15 0.5] Ces code permet de synchroniser les joueur pour une impulsion, il faudra envoyer un messager dans le server sinon les joueur type client ne pourront pas utiliser l'impulsion.
  ;;;[0.15 0.15 0.15 0.5] Replique l'impulsion pour les joueur server et Client
  (Physics|AddImpulse (Variables|Character|GetCharacterMovement) DirectionImpulse true))

(event Custom|Server%20:%20Impulse%20Speed%20Runner
  (params (DirectionImpulse :type Vector))
  ;[0 0 0 0.5 50] Gestion des mécaniquedes input
  ;;[0.15 0.15 0.15 0.5] Ces code permet de synchroniser les joueur pour une impulsion, il faudra envoyer un messager dans le server sinon les joueur type client ne pourront pas utiliser l'impulsion.
  ;;;[0.15 0.15 0.15 0.5] Replique l'impulsion pour les joueur server et Client
  (CallFunction|Client:ImpulseSpeedRunner DirectionImpulse))

(event Custom|Server%20:%20Jump
  ;[0 0 0 0.5 50] Gestion des mécaniquedes input
  ;;[0.15 0.15 0.15 0.5] Permet au joueur de faire un double jump
  (CallFunction|Client:Jump))

(event Custom|Client%20:%20Jump
  ;[0 0 0 0.5 50] Gestion des mécaniquedes input
  ;;[0.15 0.15 0.15 0.5] Permet au joueur de faire un double jump
  (Variables|/Script/Engine.MovementComponent|SetVelocity (Variables|Character|GetCharacterMovement) "0, 0, 0")
  (Physics|AddImpulse (Variables|Character|GetCharacterMovement) "0.000000,0.000000,1000.000000" true))

(event Input|EnhancedActionEvents|EnhancedInputActionIA_Jump
  (params (ActionValue :type Boolean) (ElapsedSeconds :type Float%20%28double-precision%29) (TriggeredSeconds :type Float%20%28double-precision%29) (InputAction :type Input%20Action%20Object%20Reference :default "/Game/Input/Actions/IA_Jump.IA_Jump"))
  ;[0 0 0 0.5 50] Gestion des mécaniquedes input
  ;;[0.15 0.15 0.15 0.5] Input Basic Des déplacement de personnage mes aussi
  (:Started
    (Character|Jump)
    (Class|BPIPlayer|FunctionDoubleJump(Message) self true))
  (:Canceled
    (Character|StopJumping)))

(event Input|EnhancedActionEvents|EnhancedInputActionIA_Grappin
  (params (ActionValue :type Boolean) (ElapsedSeconds :type Float%20%28double-precision%29) (TriggeredSeconds :type Float%20%28double-precision%29) (InputAction :type Input%20Action%20Object%20Reference :default "/Game/Vats/PROG/Player/Input/IA_Grappin.IA_Grappin"))
  ;[0 0 0 0.5 50] Gestion des mécaniquedes input
  ;;[0.15 0.15 0.15 0.5] Mécanique Grappin
  (:Started
    (bind _refgrappin (Variables|Actor|GetRefGrappin)
      (:then
        ;;;[0 0 0 0.5 15] Permet de détruire le grappin, ce qui a pour concéquence d'annuler les effect d'attraction vers ce dernier
        (Actor|DestroyActor _refgrappin))
      (:else
        ;;;[0.15 0.15 0.15 0.5] Code permettant d'invoquer le grappin, et d'introduire a qui appartient le grappin.
        (bind _returnvalue (Game|SpawnActorfromClass "/Game/Vats/PROG/Player/Gadget/BP_Grappin.BP_Grappin_C" (Transformation|GetWorldTransform (Variables|Default|GetArrowSpawnActor)) "Undefined" "MultiplyWithRoot" 0 self 0))
        (Variables|Actor|SetRefGrappin _returnvalue)
        ;;;[0.15 0.15 0.15 0.5] FeedBack sympatic
        (Audio|SpawnSoundAttached "/Game/Vats/Ressource/Sound/SoundGrappin/S_TireGrappin.S_TireGrappin" (Variables|Character|GetMesh) "None" "0, 0, 0" "0, 0, 0" "KeepRelativeOffset" false 1.0 1.0 0.0 0 0)))))

(event Input|EnhancedActionEvents|EnhancedInputActionIA_Move
  (params (ActionValue :type Vector%202D%20Structure) (ElapsedSeconds :type Float%20%28double-precision%29) (TriggeredSeconds :type Float%20%28double-precision%29) (InputAction :type Input%20Action%20Object%20Reference :default "/Game/Input/Actions/IA_Move.IA_Move"))
  ;[0 0 0 0.5 50] Gestion des mécaniquedes input
  ;;[0.15 0.15 0.15 0.5] Input Basic Des déplacement de personnage mes aussi
  (CallFunction|FunctionMovePlayer (.x ActionValue) (.y ActionValue)))

(event Input|EnhancedActionEvents|EnhancedInputActionIA_Interaction
  (params (ActionValue :type Boolean) (ElapsedSeconds :type Float%20%28double-precision%29) (TriggeredSeconds :type Float%20%28double-precision%29) (InputAction :type Input%20Action%20Object%20Reference :default "/Game/Vats/PROG/Player/Input/IA_Interaction.IA_Interaction"))
  ;[0 0 0 0.5 50] Gestion des mécaniquedes input
  ;;[0.15 0.15 0.15 0.5] Gestion Interaction tout objet possédant le BPI_Objet
  (:Started
    (CallFunction|FunctionInteractionObject)))

(event Input|EnhancedActionEvents|EnhancedInputActionIA_Look
  (params (ActionValue :type Vector%202D%20Structure) (ElapsedSeconds :type Float%20%28double-precision%29) (TriggeredSeconds :type Float%20%28double-precision%29) (InputAction :type Input%20Action%20Object%20Reference :default "/Game/Input/Actions/IA_Look.IA_Look"))
  ;[0 0 0 0.5 50] Gestion des mécaniquedes input
  ;;[0.15 0.15 0.15 0.5] Input Basic Des déplacement de personnage mes aussi
  (CallFunction|FunctionLook (.x ActionValue) (.y ActionValue)))

(event Input|EnhancedActionEvents|EnhancedInputActionIA_Dashing
  (params (ActionValue :type Boolean) (ElapsedSeconds :type Float%20%28double-precision%29) (TriggeredSeconds :type Float%20%28double-precision%29) (InputAction :type Input%20Action%20Object%20Reference :default "/Game/Vats/PROG/Player/Input/IA_Dashing.IA_Dashing"))
  ;[0 0 0 0.5 50] Gestion des mécaniquedes input
  ;;[0.15 0.15 0.15 0.5] Mécanique Dashing Terminer
  (:Started
    (if (>= (Variables|UseHUD|GetRechargerDashing) 3.0)
      (Variables|/Script/Engine.MovementComponent|SetVelocity (Variables|Character|GetCharacterMovement) "0, 0, 0")
      (CallFunction|Server:Dashing (* (Math|Vector|GetForwardVector (Variables|Default|GetCamera)) (Math|Conversions|ToVector(Float) 2.2e+03)))
      (Variables|Default|SetDegat_Dash true)
      (bind (_direction _chargedashing _viewcamera) (Timeline|Timeline PlayFromStart)
        (:Update
          (Variables|UseHUD|SetRechargerDashing _chargedashing)
          (Camera|SetFieldOfView (Variables|Default|GetCamera) _viewcamera))
        (:Finished
          (Variables|Default|SetDegat_Dash false))))))

(event EventBeginPlay
  ;[0 0 0 0.5 50] Gestion des mécaniquedes input
  ;;[0 0 0 0.5] Gestion des début de jeux
  (|CG_EnableMapping))

(event EventFunctionDoubleJump
  (params (TrueJumping?_FalseRest? :type Boolean))
  ;[0 0 0 0.5 50] Gestion des mécaniquedes input
  ;;[0.15 0.15 0.15 0.5] Permet au joueur de faire un double jump
  (if TrueJumping?_FalseRest?
    (if (AI|Components|NavMovement|IsFalling (Variables|Character|GetCharacterMovement))
      (Variables|Actor|GetRefGrappin
        (:then)
        (:else
          (Utilities|FlowControl|DoOnce false :!label _label
            (:Completed
              (CallFunction|Server:Jump))))))
    (else
      (goto _label Reset))))

(event EventFunctionAddCoins
  ;[0 0 0 0.5 50] Gestion des mécaniquedes input
  ;;[0.15 0.15 0.15 0.5] Input Basic Des déplacement de personnage mes aussi
  (bind _asps_player_state (Utilities|Casting|CastToPS_PlayerState (Variables|GetPlayerState)))
  (Default|CEAddCoint:Server _asps_player_state))

(event EventFunctionSpeedRunner
  (params (DirectionImpulse :type Vector :default "0, 0, 0"))
  ;[0 0 0 0.5 50] Gestion des mécaniquedes input
  ;;[0.15 0.15 0.15 0.5] Ces code permet de synchroniser les joueur pour une impulsion, il faudra envoyer un messager dans le server sinon les joueur type client ne pourront pas utiliser l'impulsion.
  (CallFunction|Server:ImpulseSpeedRunner DirectionImpulse)
  ;;;[0.15 0.15 0.15 0.5] Bonus, ce code modifie la vision du joueur.
  (bind _viewcamera (Timeline|TimelineSpeedRunner PlayFromStart)
    (:Update
      (Camera|SetFieldOfView (Variables|Default|GetCamera) _viewcamera))))

(event EventFunctionImpulsionGrappin
  (params (ForwardActor :type Vector :default "0, 0, 0"))
  ;[0 0 0 0.5 50] Gestion des mécaniquedes input
  ;;[0.15 0.15 0.15 0.5] Mécanique Grappin
  ;;;[0.15 0.15 0.15 0.5] Ce code permet d'attirer le joueur vers le grappin et impulser on direction de la camera, ATTENTION ceci ce répéter avec l'évent Tick du BP_Grappin
  ;;;;[0.15 0.15 0.15 0.5] Utiliser par le BP Grappin
  (CallFunction|Server:GrappinImpulsionPlayer ForwardActor))

(event EventFunctionDegats
  (params (PointDegat :type Integer))
  ;[0 0 0 0.5 50] ALL Gestion des Degats
  ;;[0 0 0 0.5] Gestion des dégats de sois même
  (Utilities|FlowControl|DoOnce false
    (:Completed
      (Utilities|MDegat PointDegat
        (:Dead
          (bind (_direction _deadrespawn _feedback) (Timeline|Timeline_Dead PlayFromStart)
            (:Update
              (Camera|SetFieldOfView (Variables|Default|GetCamera) _deadrespawn)
              (bind _ref_hud (Variables|UseHUD|GetREF_HUD)
                (:then
                  (Variables|/Script/UMG.Border|SetBrushColor (Variables|/Game/Vats/PROG/Player/InfosPlayer/HUD_Player.HUD_Player_C|GetBorder_FeedBack_Degat _ref_hud) (Utilities|Struct|MakeLinearColor 0.0 0.0 0.0 _feedback)))
                (:else)))
            (:Finished
              (CallFunction|CERespawn)
              (Utilities|FlowControl|Delay 2.0)
              (CallFunction|ResetDoONceDamage))))
        (:No_Dead
          (bind (_direction_2 _degats _durée_d_invincibiliter) (Timeline|Timeline_Degats PlayFromStart)
            (:Update
              (bind _ref_hud_2 (Variables|UseHUD|GetREF_HUD)
                (:then
                  (Variables|/Script/UMG.Border|SetBrushColor (Variables|/Game/Vats/PROG/Player/InfosPlayer/HUD_Player.HUD_Player_C|GetBorder_FeedBack_Degat _ref_hud_2) (Utilities|Struct|MakeLinearColor 1.0 1.0 1.0 _degats))
                  (bind _ps_player_state (Variables|UseHUD|GetPS%20Player%20State)
                    (:then
                      (Variables|/Game/Vats/PROG/Player/InfosPlayer/PS_PlayerState.PS_PlayerState_C|SetInvincible _ps_player_state _durée_d_invincibiliter))
                    (:else)))
                (:else)))
            (:Finished
              (CallFunction|ResetDoONceDamage))))))))

(fn ConstructionScript)

(fn FunctionMovePlayer
  (params (Gauche/Droite :type Float%20%28single-precision%29) (Avance/Recule :type Float%20%28single-precision%29))
  ;[0.15 0.15 0.15 0.5 15] Gestion des mouvement du joueur, en fonction de la rotation de la camera les valeur de déplacement seras modifier en concéquence
  (Pawn|Input|AddMovementInput (Math|Vector|GetRightVector (Variables|Default|GetCamera)) Gauche/Droite false)
  (Pawn|Input|AddMovementInput (Math|Vector|GetForwardVector (Variables|Default|GetCamera)) Avance/Recule false))

(fn FunctionLook
  (params (Gauche/Droite :type Float%20%28double-precision%29) (Haut/Bas :type Float%20%28double-precision%29))
  ;[0.15 0.15 0.15 0.5] Gestion de la rotation de la camera
  (Pawn|Input|AddControllerYawInput Gauche/Droite)
  (Pawn|Input|AddControllerPitchInput Haut/Bas))

(fn FunctionInteractionObject
  (bind _objet_interaction_par_bpi_object (Variables|Actor|GetObjet_Interaction_Par_BPI_Object)
    (:then
      (if (Utilities|DoesObjectImplementInterface _objet_interaction_par_bpi_object "/Game/Vats/PROG/Objet/BPI_Objet.BPI_Objet_C")
        (Class|BPIObjet|FunctionInteraction(Message) _objet_interaction_par_bpi_object)
        (Development|PrintString "Hello")))
    (:else)))

(fn FunctionVerifieLaVelocity
  (params (Actor :type Actor%20Object%20Reference))
  ;[0.15 0.15 0.15 0.5] Infliger des degats sur les joueurs [Attention pas encore installer completement]
  (Utilities|Casting|CastToBP_Piece Actor
    (:CastFailed
      (if (and (== Actor "BP_Player") (Variables|Default|GetDegat_Dash))
        (Class|BPIPlayer|FunctionDegats(Message) Actor 3)
        (else
          ;[0.15 0.15 0.15 0.5] Degat s'implique par soi même, Dash sur un mur, bonjour les dégats
          (if (>= (Math|Vector|VectorLength (Variables|/Script/Engine.MovementComponent|GetVelocity (Variables|Character|GetCharacterMovement))) 6e+02)
            (Class|BPIPlayer|FunctionDegats(Message) self 1)
            (Development|PrintString (Utilities|String|ToString(Text) (Utilities|Text|FormatText "Actor {A} Vitesse : {s}" (Math|Vector|VectorLength (Variables|/Script/Engine.MovementComponent|GetVelocity (Variables|Character|GetCharacterMovement))) Actor)))))))))