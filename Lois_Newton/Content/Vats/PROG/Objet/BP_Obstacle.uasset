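; BP_Obstacle is a tower obstacle with a platform and sphere that carries a spawned BP_Piece coin.
; On BeginPlay, Server-to-Client event pairs apply server-held scale and one of three outline materials, then spawn the piece.
; The piece gets a reference to the obstacle, attaches to the sphere at a randomized offset, and a DoOnce gate resets half a second later.
; The random size and material functions are called only from disconnected leftover nodes.
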(event Custom|Server%20:%20SpawnPiece
  (params (DoOnceTrue :type Boolean))
  ;[0.15 0.15 0.15 0.5] Ce code permet d'invoquer un BP_Piece
  (CallFunction|Client:SpawnPiece DoOnceTrue))

(event Custom|Client%20:%20SpawnPiece
  (params (Condition :type Boolean))
  ;[0.15 0.15 0.15 0.5] Ce code permet d'invoquer un BP_Piece
  (if Condition
    (Utilities|FlowControl|DoOnce false :!label _label
      (:Completed
        (bind _returnvalue (Game|SpawnActorfromClass "/Game/Vats/PROG/Objet/BP_Piece.BP_Piece_C" (Math|Transform|MakeTransform (Transformation|GetActorLocation) "0, 0, 0" "1.000000,1.000000,1.000000") "Undefined" "MultiplyWithRoot" 0 self 0))
        (bind _output_get (Variables|Default|SetPiece _returnvalue))
        (Transformation|AttachComponentToComponent _output_get (Variables|Default|GetSphere%20:%20Tour) "None" "KeepRelative" "KeepRelative" "KeepRelative" true)
        (Transformation|SetActorRelativeLocation (Variables|Default|GetPiece) (Math|Vector|MakeVector (select (Math|Random|RandomBool) 3e+02 -3e+02) (select (Math|Random|RandomBool) 3e+02 -3e+02) (Math|Random|RandomFloatinRange -1.5e+03 2e+02)) false true)
        (Utilities|FlowControl|Delay 0.5)
        (CallFunction|Server:SpawnPiece false)))
    (else
      (goto _label Reset))))

(event Custom|Client%20:%20Replicate
  (bind _server___scaleobject (Variables|Default|GetServer%20:%20ScaleObject))
  (bind _server___scaleobject_2 (Variables|Default|GetServer%20:%20ScaleObject))
  (bind _server___integrationmaterial (Variables|Default|GetServer%20:%20IntegrationMaterial))
  (bind _returnvalue (Utilities|Select :Index _server___integrationmaterial :Option%200 "/Game/Vats/Ressource/CustomMaterial/OutlinePlayer/MI_TourOutline/MI_Outline_Tour_01.MI_Outline_Tour_01" :Option%201 "/Game/Vats/Ressource/CustomMaterial/OutlinePlayer/MI_TourOutline/MI_Outline_Tour_02.MI_Outline_Tour_02" :Option%202 "/Game/Vats/Ressource/CustomMaterial/OutlinePlayer/MI_TourOutline/MI_Outline_Tour_03.MI_Outline_Tour_03"))
  ;[0.15 0.15 0.15 0.5] Gestion des Obstacle
  (Transformation|SetRelativeScale3D (Variables|Default|GetObstacle) (Math|Vector|MakeVector (.x _server___scaleobject) (.y _server___scaleobject) (.z _server___scaleobject)))
  (Transformation|SetRelativeScale3D (Variables|Default|GetPlateforme) (Math|Vector|MakeVector (+ (.x _server___scaleobject_2) 1.0) (+ (.y _server___scaleobject_2) 1.0) 0.1))
  (Transformation|SetWorldScale3D (Variables|Default|GetSphere%20:%20Tour) "1.000000,1.000000,1.000000")
  ;[0.15 0.15 0.15 0.5] Gestion Random Color
  (Rendering|Material|SetMaterial (Variables|Default|GetObstacle) 0 _returnvalue)
  (Rendering|Material|SetMaterial (Variables|Default|GetSphere%20:%20Tour) 0 _returnvalue)
  (Rendering|Material|SetMaterial (Variables|Default|GetPlateforme) 0 _returnvalue))

(event Custom|Server%20:%20Replicate
  ;[0.15 0.15 0.15 0.5] Gestion des Obstacle
  (CallFunction|Client:Replicate))

(event EventBeginPlay
  (CallFunction|Server:Replicate)
  (CallFunction|Server:SpawnPiece true))

(fn ConstructionScript)

(fn FunctionGestionTaille
  (bind _returnvalue (Math|Random|RandomFloatinRange 0.3 1.5))
  (bind _returnvalue_2 (Math|Random|RandomFloatinRange 0.3 1.5))
  (Transformation|SetRelativeScale3D (Variables|Default|GetObstacle) (Math|Vector|MakeVector _returnvalue _returnvalue_2 (Math|Random|RandomFloatinRange 5.0 15.0)))
  (Transformation|SetRelativeScale3D (Variables|Default|GetPlateforme) (Math|Vector|MakeVector (+ _returnvalue 1.0) (+ _returnvalue_2 1.0) 0.1))
  (Transformation|SetWorldScale3D (Variables|Default|GetSphere%20:%20Tour) "1.000000,1.000000,1.000000"))

(fn FunctionSetMaterial
  (params (Material :type Material%20Interface%20Object%20Reference))
  (Rendering|Material|SetMaterial (Variables|Default|GetObstacle) 0 Material)
  (Rendering|Material|SetMaterial (Variables|Default|GetSphere%20:%20Tour) 0 Material)
  (Rendering|Material|SetMaterial (Variables|Default|GetPlateforme) 0 Material))