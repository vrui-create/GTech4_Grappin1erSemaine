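; BP_Piece is a collectible coin that awards the player and restores their mid-air jump.
; A Timeline animates the mesh's height and yaw, replacing an Animation Blueprint.
; On sphere overlap with a BPI_Player actor, a DoOnce sends coin and double-jump interface messages and spawns VFX and sound.
; It asks its referenced obstacle, if valid, to spawn a piece via ServerSpawnPiece, then destroys itself after a short delay.
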(event OnComponentBeginOverlap(Sphere)
  (params (OverlappedComponent :type Primitive%20Component%20Object%20Reference) (OtherActor :type Actor%20Object%20Reference) (OtherComp :type Primitive%20Component%20Object%20Reference) (OtherBodyIndex :type Integer) (bFromSweep :type Boolean) (SweepResult :type Hit%20Result%20Structure%20%28by%20ref%29))
  ;[0.15 0.15 0.15 0.5] En entrant dans la piece le joueur récupérer une piéce, un FeedBack Visuel & Auditif, qui confirmer que l'objet est récuperer
  (if (Utilities|DoesObjectImplementInterface OtherActor "/Game/Vats/PROG/Player/BPI_Player.BPI_Player_C")
    ;;[0.15 0.15 0.15 0.5 15] Do once permet de lancée qu'une fois la séquence. Elle peut se réutiliser qu'a condition qu'une autre s'attacher au reset
    (Utilities|FlowControl|DoOnce false
      (:Completed
        ;;[0.15 0.15 0.15 0.5 15] FeedBack, permet d'afficher un évenement visuel ou auditif. Pour nous, elle confirmeras au prés des joueur que l'objet est ramasser
        (CallFunction|FunctionFeedBackCoins OtherActor)
        ;;[0.15 0.15 0.15 0.5] Auto destruction, permet de supprimer un objet dans le monde afin d'économiser de la place
        (Utilities|FlowControl|Delay 0.1)
        (Actor|DestroyActor)))))

(event EventBeginPlay
  ;[0.15 0.15 0.15 0.5] Ce code permet de faire tourner la piece sans utiliser un ABP_Animation
  (bind (_direction _relativelocate_z _relativerotation_z) (Timeline|Timeline PlayFromStart)
    (:Update
      (Transformation|SetRelativeLocationAndRotation (Variables|Default|GetStaticMesh) (Math|Vector|MakeVector 0.0 0.0 _relativelocate_z) (Math|Rotator|MakeRotator 0.0 0.0 _relativerotation_z) true false))))

(fn ConstructionScript)

(fn FunctionFeedBackCoins
  (params (ActorDectected :type Actor%20Object%20Reference))
  (bind _returnvalue (Transformation|GetActorTransform))
  ;[0.15 0.15 0.15 0.5 15] BPI Interface, Permet au d'ajouter au player des poins dans le player state
  (Class|BPIPlayer|FunctionAddCoins(Message) ActorDectected)
  ;[0.15 0.15 0.15 0.5 15] Permet au joueur d'utiliser a nouveau son jump en plein air
  (Class|BPIPlayer|FunctionDoubleJump(Message) ActorDectected false)
  ;[0.15 0.15 0.15 0.5] FeedBack : ce code permet de valider visuellement et auditivement, que la piéce est bien pris
  (Niagara|SpawnSystematLocation "/Game/Vats/Ressource/VFX/VFX_Coins.VFX_Coins" (.location _returnvalue) (.rotation _returnvalue))
  (Audio|SpawnSoundatLocation "/Game/Vats/Ressource/Sound/Music_Background/SoundCoins/SC_Coins.SC_Coins" (Transformation|GetActorLocation) "0, 0, 0" 1.0 1.0 0.0 0 0)
  ;[0.15 0.15 0.15 0.5] Ce code permet de réinvoquer une piece dans le BP_Obstacle
  (bind _ref_obstacle (Variables|Default|GetREF_Obstacle)
    (:then
      (Default|Server:SpawnPiece _ref_obstacle true))
    (:else)))