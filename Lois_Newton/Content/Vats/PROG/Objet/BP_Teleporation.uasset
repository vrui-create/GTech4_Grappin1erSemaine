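; Interactable end-of-level teleporter that either moves the player to a target actor or opens the start menu level, as set by a flag that also picks its label.
; A sphere overlap shows the widget and registers the object on the player for interface-driven interaction.
; Interaction animates the camera FOV with a timeline before acting, with a second FOV timeline after teleporting.
; The widget turns toward the player every tick.
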(event OnComponentBeginOverlap(Sphere)
  (params (OverlappedComponent :type Primitive%20Component%20Object%20Reference) (OtherActor :type Actor%20Object%20Reference) (OtherComp :type Primitive%20Component%20Object%20Reference) (OtherBodyIndex :type Integer) (bFromSweep :type Boolean) (SweepResult :type Hit%20Result%20Structure%20%28by%20ref%29))
  ;[0.15 0.15 0.15 0.5] Rendre le widget [Visible/Invisible] en fonction du joueur
  (Utilities|MVisibleJoueur OtherActor true))

(event OnComponentEndOverlap(Sphere)
  (params (OverlappedComponent :type Primitive%20Component%20Object%20Reference) (OtherActor :type Actor%20Object%20Reference) (OtherComp :type Primitive%20Component%20Object%20Reference) (OtherBodyIndex :type Integer))
  ;[0.15 0.15 0.15 0.5] Rendre le widget [Visible/Invisible] en fonction du joueur
  (Utilities|MVisibleJoueur OtherActor false))

(event EventTick
  (params (DeltaSeconds :type Float%20%28single-precision%29))
  ;[0.15 0.15 0.15 0.5] tourne automatiquement le widget vers le joueur
  (CallFunction|FunctionRotationWidget))

(event EventFunctionInteraction
  ;[0 0 0 0.5] Interaction BPI_Objet permet au joueur de faire une interaction sur les objet
  ;;[0.15 0.15 0.15 0.5] Modifie la vue du joueur
  (bind _viewcamera (Timeline|Timeline PlayFromStart)
    (:Update
      (Camera|SetFieldOfView (Variables|/Game/Vats/PROG/Player/BP_Player.BP_Player_C|GetCamera (Variables|Default|GetBP_Player)) _viewcamera))
    (:Finished
      (if (Variables|Default|GetTeleportation%20/%20Fin%20Niveau)
        ;;[0.15 0.15 0.15 0.5] Cette partie permet de teleporter le joueur Vers un actor
        (bind _target_teleportation (Variables|Default|GetTarget_Teleportation)
          (:then
            (Transformation|SetActorLocationAndRotation (Game|GetPlayerCharacter 0) (.location (Transformation|GetActorTransform _target_teleportation)) (.rotation (Transformation|GetActorTransform _target_teleportation)) false true)
            ;;[0.15 0.15 0.15 0.5] Modifie la vue du joueur
            (bind _viewcamera_2 (Timeline|Timeline_0 PlayFromStart)
              (:Update
                (Camera|SetFieldOfView (Variables|/Game/Vats/PROG/Player/BP_Player.BP_Player_C|GetCamera (Variables|Default|GetBP_Player)) _viewcamera_2))))
          (:else))
        (else
          ;;[0.15 0.15 0.15 0.5] Fin Niveau
          (Game|OpenLevel(byObjectReference) "/Game/Vats/MAP/MenueStart.MenueStart"))))))

(event EventBeginPlay
  ;[0.15 0.15 0.15 0.5] Initialize le player
  (Rendering|Components|TextRender|SetText (Variables|Default|GetTextRender) (Utilities|Text|FormatText (select (Variables|Default|GetTeleportation%20/%20Fin%20Niveau) "Prochain Niveau" "Fin Niveau")))
  (bind _asbp_player (Utilities|Casting|CastToBP_Player (Game|GetPlayerCharacter 0)))
  (Variables|Default|SetBP_Player _asbp_player))

(fn ConstructionScript)

(fn FunctionRotationWidget
  (bind _returnvalue (Game|GetPlayerCharacter 0))
  (Utilities|IsValid _returnvalue
    (:Is%20Valid
      (Transformation|SetWorldRotation (Variables|Default|GetWidget) (Math|Rotator|FindLookatRotation (Transformation|GetWorldLocation (Variables|Default|GetWidget)) (Transformation|GetActorLocation _returnvalue)) false false))))